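; BP_PhysicsPickup is an interactable cube that players pick up and drop through interact events.
; On interact, if the player is not holding, it disables physics and collision and attaches the Cube to the player's Arrow1, leaving IsHolding false.
; Drop detaches the actor rather than the Cube component, keeping world transform, and leaves physics and collision disabled.
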(event `/Game/Interfaces/Interface_interact.INT_Interact`
  (params (PlayerRef :type "/Game/Player/BP_PlayerChar Object Reference"))
  (bind _cube (`self.Cube`))
  (if (not (`/Game/Player/BP_PlayerChar.isHolding?` PlayerRef))
    (set `/Game/Player/BP_PlayerChar.isHolding?` false PlayerRef)
    (`PrimitiveComponent.SetSimulatePhysics` _cube false)
    (`PrimitiveComponent.SetCollisionEnabled` _cube "NoCollision")
    (`SceneComponent.K2_AttachToComponent` (`self.Cube`) (`/Game/Player/BP_PlayerChar.Arrow1` PlayerRef) "None" "SnapToTarget" "KeepRelative" "KeepRelative" true)))

(event `/Game/Interfaces/Interface_interact.INT_Drop`
  (bind _cube (`self.Cube`))
  (`self.K2_DetachFromActor` "KeepWorld" "KeepWorld" "KeepWorld")
  (`PrimitiveComponent.SetCollisionEnabled` _cube "NoCollision")
  (`PrimitiveComponent.SetSimulatePhysics` _cube false))

(fn `UserConstructionScript`)